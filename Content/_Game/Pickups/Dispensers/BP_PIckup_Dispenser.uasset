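; Pickup dispenser that spawns a sequence of pickup actors from an array at its spawn location, one at a time.
; Tick waits a spawn delay, spawns the current entry and activates the sphere.
; When a BP_ShooterCharacter stops overlapping the sphere, it deactivates the sphere and advances the index to allow the next spawn.
; Once the array runs out, the sphere is destroyed, halting further spawns.
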(event `self.ReceiveTick`
  (params (DeltaSeconds :type "Float (single-precision)"))
  (bind _sphere (`self.Sphere`))
  (bind _nextpickupindex (`self.NextPickupIndex`))
  (bind _pickuparray (`self.PickupArray`))
  ;[1 1 1] If Conditions are met, Spawn the Next Pickup Type
  (if (`KismetSystemLibrary.IsValid` (`self.Sphere`))
    (if (`self.PickupSpawned`)
      _
      (elif (`self.Expired`)
        (`ActorComponent.Deactivate` (`self.DefaultSceneRoot`))
        (else
          (`KismetSystemLibrary.Delay` (`self.SpawnDuration`))
          (if (< _nextpickupindex (`KismetArrayLibrary.Array_Length` _pickuparray))
            (`|SpawnActorFromClass` (`|GetArrayItem` _pickuparray _nextpickupindex) (`KismetMathLibrary.Conv_VectorToTransform` (`SceneComponent.K2_GetComponentLocation` (`self.SpawnLocation`))) "Undefined" "OverrideRootScale" null null)
            (set `self.PickupSpawned` true)
            (`/Engine/EditorBlueprintResources/StandardMacros.IsValid` _sphere
              (:`Is Valid`
                (`ActorComponent.Activate` _sphere false)))
            (else
              (`ActorComponent.K2_DestroyComponent` (`self.Sphere`)))))))))

(event `self.Sphere.OnComponentEndOverlap`
  (params (OverlappedComponent :type "PrimitiveComponent Object Reference") (OtherActor :type "Actor Object Reference") (OtherComp :type "PrimitiveComponent Object Reference") (OtherBodyIndex :type Integer))
  ;[1 1 1] On End Overlap Increment to Next Pickup Type in Array
  (if (`self.PickupSpawned`)
    (cast `/Game/_Game/Characters/BP_ShooterCharacter` OtherActor)
    (`ActorComponent.Deactivate` (`self.Sphere`))
    (if (<= (`self.NextPickupIndex`) (- (`KismetArrayLibrary.Array_Length` (`self.PickupArray`)) 1))
      (set `self.NextPickupIndex` (+ (`self.NextPickupIndex`) 1))
      (set `self.PickupSpawned` false)
      (else
        (`ActorComponent.K2_DestroyComponent` (`self.Sphere`))
        (set `self.Expired` true)))))

(fn `UserConstructionScript`)