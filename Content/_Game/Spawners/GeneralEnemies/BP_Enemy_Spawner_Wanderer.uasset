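; Enemy spawner that places randomly chosen actors from a class list at its spawn location, restricted to day, night or both by flags.
; Tick checks the day/night state, then uses latent Delays for an initial wait before the first spawn and a cooldown before each spawn.
; The spawner counts successful spawns and destroys itself at the maximum, or when a spawn fails, including when collision adjustment finds no free spot.
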(event `self.ReceiveTick`
  (params (DeltaSeconds :type "Float (single-precision)"))
  (bind _actorclasses (`self.ActorClasses`))
  ;[1 1 1] Spawn Enemy Grux on each cooldown until maxspawn limit reached
  (if (or (and (`self.SpawnAtNight`) (not (`/Game/_Game/FunctionLibraries/FNL_Enemy.GetDayNight`))) (and (`self.SpawnAtDay`) (`/Game/_Game/FunctionLibraries/FNL_Enemy.GetDayNight`)))
    (if (== (`self.SpawnCount`) 0)
      (`KismetSystemLibrary.Delay` (`self.InitialDelay`)))
    (if (>= (`self.SpawnCount`) (`self.MaximumSpawns`))
      (`self.K2_DestroyActor`)
      (else
        (`KismetSystemLibrary.Delay` (`self.Spawn Cooldown`))
        (bind _returnvalue (`|SpawnActorFromClass` (`|GetArrayItem` _actorclasses (`KismetMathLibrary.RandomIntegerInRange` 0 (- (`KismetArrayLibrary.Array_Length` _actorclasses) 1))) (`KismetMathLibrary.Conv_VectorToTransform` (`SceneComponent.K2_GetComponentLocation` (`self.SpawnLocation`))) "AdjustIfPossibleButDontSpawnIfColliding" "OverrideRootScale" null null))
        (`/Engine/EditorBlueprintResources/StandardMacros.IsValid` _returnvalue
          (:`Is Valid`
            (set `self.SpawnCount` (+ (`self.SpawnCount`) 1)))
          (:`Is Not Valid`
            (`self.K2_DestroyActor`)))))))

(fn `UserConstructionScript`)