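; Blood Rage Grux enemy Blueprint that handles the enemy's on-screen UI feedback, a health bar and floating hit numbers.
; BeginPlay links the health bar widget to this enemy and hides it, leaving Show and Hide events to toggle visibility.
; When allowed, hits spawn an animated number widget at the projected screen position, showing damage and headshot state and registered through StoreHitNumber with its world location.
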(event `self.ReceiveBeginPlay`
  ;[1 1 1] Begin Play
  (`parent.ReceiveBeginPlay`)
  (bind _aswbp_enemy_health_bar (cast `/Game/_Game/HUD/WBP_EnemyHealthBar` (`WidgetComponent.GetUserWidgetObject` (`self.HealthBar`))))
  (set `/Game/_Game/HUD/WBP_EnemyHealthBar.Enemy` self _aswbp_enemy_health_bar)
  (`Widget.SetVisibility` (`WidgetComponent.GetUserWidgetObject` (`self.HealthBar`)) "Hidden"))

(event `self.ShowHealthBar`
  ;[1 1 1] This Blueprint Implementable event calls the parent version of ShowHealthBar_implementation()
  (`Widget.SetVisibility` (`WidgetComponent.GetUserWidgetObject` (`self.HealthBar`)) "Visible")
  (`parent.ShowHealthBar`))

(event `self.HideHealthBar`
  ;[1 1 1] Hide Health Bar
  (`Widget.SetVisibility` (`WidgetComponent.GetUserWidgetObject` (`self.HealthBar`)) "Hidden"))

(event `self.ShowHitNumber`
  (params (Damage :type Integer) (HitLocation :type "Vector Structure") (bHeadShot :type Boolean) (bCriticalHit :type Boolean))
  (if (`/Game/_Game/FunctionLibraries/FNL_Enemy.ShouldShowHitNumbers` self)
    (bind _returnvalue (`|CreateWidget` "/Game/_Game/HUD/WBP_HitNumbers.WBP_HitNumbers_C"))
    (`UserWidget.AddToViewport` _returnvalue 0)
    (`UserWidget.SetPositionInViewport` _returnvalue (`GameplayStatics.ProjectWorldToScreen` (`GameplayStatics.GetPlayerController` 0) HitLocation) true)
    (`self.StoreHitNumber` _returnvalue HitLocation)
    (set `/Game/_Game/HUD/WBP_HitNumbers.HitText` (`KismetTextLibrary.Conv_IntToText` Damage) _returnvalue)
    (set `/Game/_Game/HUD/WBP_HitNumbers.HeadShot` bHeadShot _returnvalue)
    (`UserWidget.PlayAnimation` _returnvalue (`/Game/_Game/HUD/WBP_HitNumbers.HitNumberAnimation` _returnvalue) 0.0 1 "Forward" 1.0 false)))

(fn `UserConstructionScript`)