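; Floating sapphire ecosystem Blueprint that fades its light with the day/night cycle.
; Every Tick it polls GetDayNight and plays a timeline forward when true or reverses it when false.
; The timeline value, scaled by IlluminationMultiplier, sets the light intensity.
; A Completed flag is set on each poll and cleared when the timeline finishes, but this graph never reads it.
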(event `self.ReceiveTick`
  (params (DeltaSeconds :type "Float (single-precision)"))
  (if (`/Game/_Game/FunctionLibraries/FNL_Enemy.GetDayNight`)
    (set `self.Completed` true)
    (bind (_direction _newtrack_0) (`Timeline|Timeline_0` :!label _label)
      (:`Update`
        (`KismetSystemLibrary.PrintString` (`KismetStringLibrary.Conv_DoubleToString` _newtrack_0) false false (struct :`R` 1.0 :`G` 0.844085 :`A` 1.0) 0.5)
        (`LightComponent.SetIntensity` (`self.Light`) (* _newtrack_0 (`self.IlluminationMultiplier`))))
      (:`Finished`
        (set `self.Completed` false)
        (`KismetSystemLibrary.PrintString` "Day Completed" false false (struct :`R` 1.0 :`B` 0.040396 :`A` 1.0) 5.0)))
    (else
      (set `self.Completed` true)
      (goto _label :!via `Reverse`))))

(fn `UserConstructionScript`)