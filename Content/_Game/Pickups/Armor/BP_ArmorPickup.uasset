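; BP_ArmorPickup is a pickup that grants armor to the shooter character that touches it.
; On sphere overlap it adds ArmorAmount to the character's Armor, capped at MaxArmor.
; It then plays a pickup sound at the character, attaches a particle effect to the character's capsule and destroys itself, even if armor was already full.
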(event `self.Sphere.OnComponentBeginOverlap`
  (params (OverlappedComponent :type "PrimitiveComponent Object Reference") (OtherActor :type "Actor Object Reference") (OtherComp :type "PrimitiveComponent Object Reference") (OtherBodyIndex :type Integer) (bFromSweep :type Boolean) (SweepResult :type "HitResult Structure (by ref)"))
  (bind _asbp_shooter_character (cast `/Game/_Game/Characters/BP_ShooterCharacter` OtherActor))
  (bind _returnvalue (+ (`self.ArmorAmount`) (`ShooterCharacter.Armor` _asbp_shooter_character)))
  (bind _maxarmor (`ShooterCharacter.MaxArmor` _asbp_shooter_character))
  (if (> _returnvalue _maxarmor)
    (set `ShooterCharacter.Armor` _maxarmor _asbp_shooter_character)
    (else
      (set `ShooterCharacter.Armor` _returnvalue _asbp_shooter_character)))
  (`GameplayStatics.PlaySoundAtLocation` (`self.ArmorPickupSound`) (`self.K2_GetActorLocation` _asbp_shooter_character) (struct) 1.0 1.0 0.0 null null null)
  (`GameplayStatics.SpawnEmitterAttached` "/Game/_Game/Pickups/VFX/Armor_Pick_VFX.Armor_Pick_VFX" (`Character.CapsuleComponent` _asbp_shooter_character) "None" (0.0 0.0 0.0) (struct) (1.0 1.0 1.0) "SnapToTargetIncludingScale")
  (`self.K2_DestroyActor`))

(fn `UserConstructionScript`)