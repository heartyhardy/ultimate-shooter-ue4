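; Area trigger that spawns Warchief mini-boss enemies when the player character enters, optionally restricted to day or night.
; Each entry spawns one enemy after a cooldown, with an extra initial delay before the first, and sets the player as its blackboard target.
; A gate blocks retriggering until the player exits.
; The spawner destroys itself if a spawn fails or on a qualifying entry after reaching the spawn limit.
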(event `self.Trigger.OnComponentBeginOverlap`
  (params (OverlappedComponent :type "PrimitiveComponent Object Reference") (OtherActor :type "Actor Object Reference") (OtherComp :type "PrimitiveComponent Object Reference") (OtherBodyIndex :type Integer) (bFromSweep :type Boolean) (SweepResult :type "HitResult Structure (by ref)"))
  (bind _returnvalue (`GameplayStatics.GetPlayerPawn` 0))
  ;[1 1 1] Spawn Enemy Grux on each cooldown until maxspawn limit reached
  (bind _asbp_shooter_character (cast `/Game/_Game/Characters/BP_ShooterCharacter` OtherActor))
  (`/Engine/EditorBlueprintResources/StandardMacros.IsValid` _asbp_shooter_character
    (:`Is Valid`
      ;;[1 1 1] Lock Trigger
      (if (not (`self.TriggerGated`))
        (set `self.TriggerGated` true)
        (if (or (and (`self.SpawnAtNight`) (not (`/Game/_Game/FunctionLibraries/FNL_Enemy.GetDayNight`))) (and (`self.SpawnAtDay`) (`/Game/_Game/FunctionLibraries/FNL_Enemy.GetDayNight`)))
          (if (== (`self.SpawnCount`) 0)
            (`KismetSystemLibrary.Delay` (`self.InitialDelay`)))
          (if (>= (`self.SpawnCount`) (`self.MaximumSpawns`))
            (`self.K2_DestroyActor`)
            (else
              (`KismetSystemLibrary.Delay` (`self.Spawn Cooldown`))
              (bind _returnvalue_2 (`|SpawnActorFromClass` "/Game/_Game/Enemies/Grux/BP_EnemyWarchief.BP_EnemyWarchief_C" (`KismetMathLibrary.Conv_VectorToTransform` (`SceneComponent.K2_GetComponentLocation` (`self.SpawnLocation`))) "Undefined" "OverrideRootScale" null null))
              (`/Engine/EditorBlueprintResources/StandardMacros.IsValid` _returnvalue_2
                (:`Is Valid`
                  (set `self.SpawnCount` (+ (`self.SpawnCount`) 1))
                  (`/Engine/EditorBlueprintResources/StandardMacros.IsValid` _returnvalue
                    (:`Is Valid`
                      (bind _asbp_shooter_character_2 (cast `/Game/_Game/Characters/BP_ShooterCharacter` _returnvalue))
                      (`BlackboardComponent.SetValueAsObject` (`AIBlueprintHelperLibrary.GetBlackboard` _returnvalue_2) (`self.TargetActorName`) _asbp_shooter_character_2))))
                (:`Is Not Valid`
                  (`self.K2_DestroyActor`))))))))))

(event `self.Trigger.OnComponentEndOverlap`
  (params (OverlappedComponent :type "PrimitiveComponent Object Reference") (OtherActor :type "Actor Object Reference") (OtherComp :type "PrimitiveComponent Object Reference") (OtherBodyIndex :type Integer))
  ;[1 1 1] Unlock Trigger
  (bind _asbp_shooter_character (cast `/Game/_Game/Characters/BP_ShooterCharacter` OtherActor))
  (`/Engine/EditorBlueprintResources/StandardMacros.IsValid` _asbp_shooter_character
    (:`Is Valid`
      (set `self.TriggerGated` false))))

(fn `UserConstructionScript`)