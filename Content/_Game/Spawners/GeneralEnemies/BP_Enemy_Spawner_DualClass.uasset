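; Enemy spawner actor that spawns a regular Grux by day or a Dark Lurker Grux by night, within its allowed periods.
; Tick drives latent delays for the initial wait and cooldown, then spawns at the SpawnLocation component.
; Each spawn increments the count and receives the player's shooter character as its blackboard target.
; The spawner destroys itself at the spawn limit or when a spawn fails.
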(event `self.ReceiveTick`
  (params (DeltaSeconds :type "Float (single-precision)"))
  (bind _returnvalue (`GameplayStatics.GetPlayerPawn` 0))
  (bind _targetactorname (`self.TargetActorName`))
  (bind _returnvalue_2 (`KismetMathLibrary.Conv_VectorToTransform` (`SceneComponent.K2_GetComponentLocation` (`self.SpawnLocation`))))
  ;[1 1 1] Spawn Enemy Grux on each cooldown until maxspawn limit reached
  (if (or (and (`self.SpawnAtNight`) (not (`/Game/_Game/FunctionLibraries/FNL_Enemy.GetDayNight`))) (and (`self.SpawnAtDay`) (`/Game/_Game/FunctionLibraries/FNL_Enemy.GetDayNight`)))
    (if (== (`self.SpawnCount`) 0)
      (`KismetSystemLibrary.Delay` (`self.InitialDelay`)))
    (if (>= (`self.SpawnCount`) (`self.MaximumSpawns`))
      (`self.K2_DestroyActor`)
      (else
        (`KismetSystemLibrary.Delay` (`self.Spawn Cooldown`))
        (if (`/Game/_Game/FunctionLibraries/FNL_Enemy.GetDayNight`)
          (bind _returnvalue_3 (`|SpawnActorFromClass` "/Game/_Game/Enemies/Grux/BP_EnemyGrux.BP_EnemyGrux_C" _returnvalue_2 "Undefined" "OverrideRootScale" null null))
          (`/Engine/EditorBlueprintResources/StandardMacros.IsValid` _returnvalue_3
            (:`Is Valid`
              (set `self.SpawnCount` (+ (`self.SpawnCount`) 1) :!label _label)
              (`/Engine/EditorBlueprintResources/StandardMacros.IsValid` _returnvalue
                (:`Is Valid`
                  (bind _asbp_shooter_character (cast `/Game/_Game/Characters/BP_ShooterCharacter` _returnvalue))
                  (if (`/Game/_Game/FunctionLibraries/FNL_Enemy.GetDayNight`)
                    (`BlackboardComponent.SetValueAsObject` (`AIBlueprintHelperLibrary.GetBlackboard` _returnvalue_3) _targetactorname _asbp_shooter_character)
                    (else
                      (`BlackboardComponent.SetValueAsObject` (`AIBlueprintHelperLibrary.GetBlackboard` (stale _returnvalue_4)) _targetactorname _asbp_shooter_character))))))
            (:`Is Not Valid`
              (`self.K2_DestroyActor`)))
          (else
            (bind _returnvalue_4 (`|SpawnActorFromClass` "/Game/_Game/Enemies/Grux/BP_EnemyGrux_DarkLurker.BP_EnemyGrux_DarkLurker_C" _returnvalue_2 "Undefined" "OverrideRootScale" null null))
            (`/Engine/EditorBlueprintResources/StandardMacros.IsValid` _returnvalue_4
              (:`Is Valid`
                (goto _label))
              (:`Is Not Valid`
                (`self.K2_DestroyActor`)))))))))

(fn `UserConstructionScript`)