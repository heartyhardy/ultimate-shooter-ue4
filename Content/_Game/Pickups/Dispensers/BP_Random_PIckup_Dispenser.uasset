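; BP_Random_PIckup_Dispenser is a pickup dispenser that spawns randomly chosen pickups from a class array.
; Tick polls while no pickup is out, waits through a Delay, then spawns the indexed class at SpawnLocation and activates the Sphere.
; When a BP_ShooterCharacter ends overlap with the Sphere after a spawn, it deactivates the Sphere, randomizes the next index and clears the spawned flag, restarting the cycle.
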(event `self.ReceiveTick`
  (params (DeltaSeconds :type "Float (single-precision)"))
  (bind _sphere (`self.Sphere`))
  ;[1 1 1] If Conditions are met, Spawn the Next Pickup Type
  (if (`KismetSystemLibrary.IsValid` (`self.Sphere`))
    (if (not (`self.PickupSpawned`))
      (`KismetSystemLibrary.Delay` (`self.SpawnDuration`))
      (`|SpawnActorFromClass` (`|GetArrayItem` (`self.PickupArray`) (`self.NextPickupIndex`)) (`KismetMathLibrary.Conv_VectorToTransform` (`SceneComponent.K2_GetComponentLocation` (`self.SpawnLocation`))) "Undefined" "OverrideRootScale" null null)
      (set `self.PickupSpawned` true)
      (`/Engine/EditorBlueprintResources/StandardMacros.IsValid` _sphere
        (:`Is Valid`
          (`ActorComponent.Activate` _sphere false))))))

(event `self.Sphere.OnComponentEndOverlap`
  (params (OverlappedComponent :type "PrimitiveComponent Object Reference") (OtherActor :type "Actor Object Reference") (OtherComp :type "PrimitiveComponent Object Reference") (OtherBodyIndex :type Integer))
  ;[1 1 1] On End Overlap Increment to Next Pickup Type in Array
  (if (`self.PickupSpawned`)
    (cast `/Game/_Game/Characters/BP_ShooterCharacter` OtherActor)
    (`ActorComponent.Deactivate` (`self.Sphere`))
    (set `self.NextPickupIndex` (`KismetMathLibrary.RandomIntegerInRange` 0 (- (`KismetArrayLibrary.Array_Length` (`self.PickupArray`)) 1)))
    (set `self.PickupSpawned` false)))

(fn `UserConstructionScript`)