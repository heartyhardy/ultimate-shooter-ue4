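; Speed pickup that grants a timed movement speed bonus to a BP_ShooterCharacter overlapping its sphere.
; On overlap it sets the character's bonus speed modifier, plays a pickup sound and burst effect, and activates a looping buff effect on the character's persistent effect component.
; After a short delay it looks up BP_Announcer, triggers the speed buff announcement and destroys itself, both only if an announcer exists.
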(event `self.Sphere.OnComponentBeginOverlap`
  (params (OverlappedComponent :type "PrimitiveComponent Object Reference") (OtherActor :type "Actor Object Reference") (OtherComp :type "PrimitiveComponent Object Reference") (OtherBodyIndex :type Integer) (bFromSweep :type Boolean) (SweepResult :type "HitResult Structure (by ref)"))
  (bind _asbp_shooter_character (cast `/Game/_Game/Characters/BP_ShooterCharacter` OtherActor))
  (`ShooterCharacter.SetBonusSpeedModifierTimed` _asbp_shooter_character (`self.SpeedAmount`) (`self.SpeedTimeout`))
  (`GameplayStatics.PlaySoundAtLocation` (`self.SpeedPickupSound`) (`self.K2_GetActorLocation` _asbp_shooter_character) (struct) 1.0 1.0 0.0 null null null)
  (`GameplayStatics.SpawnEmitterAttached` "/Game/_Game/Pickups/VFX/Speed_Pick_VFX.Speed_Pick_VFX" (`Character.CapsuleComponent` _asbp_shooter_character) "None" (0.0 0.0 0.0) (struct) (1.0 1.0 1.0) "SnapToTargetIncludingScale")
  (bind _pickuppersistenteffect (`ShooterCharacter.PickupPersistentEffect` _asbp_shooter_character))
  (`ParticleSystemComponent.SetTemplate` _pickuppersistenteffect "/Game/_Game/Pickups/VFX/Speed_Bonus_VFX_Loop.Speed_Bonus_VFX_Loop")
  (`ActorComponent.Activate` _pickuppersistenteffect false)
  (`KismetSystemLibrary.Delay` 0.3)
  ;[1 1 1] Announcer Buff Damage
  (bind _returnvalue (`GameplayStatics.GetActorOfClass` "/Game/_Game/Announcer/BP_Announcer.BP_Announcer_C"))
  (`/Engine/EditorBlueprintResources/StandardMacros.IsValid` _returnvalue
    (:`Is Valid`
      (`Announcer.PlaySpeedBuffAnnouncement` _returnvalue)
      (`self.K2_DestroyActor`))))

(fn `UserConstructionScript`)